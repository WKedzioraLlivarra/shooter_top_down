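; BP_Spider is an enemy spider that chases the player and attacks in melee.
; From BeginPlay it reissues an AI MoveTo toward the player character every 0.2 seconds.
; Tick checks the distance against AttackRange and, when no attack montage is playing, deactivates character movement and plays AN_SpiderAttack.
; Movement reactivates when the montage completes, and the file itself applies no damage.
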(event `self.ReceiveBeginPlay`
  (`|AIMoveTo` self (0.0 0.0 0.0) (`GameplayStatics.GetPlayerCharacter` 0) :!label _label
    (:`then`
      (`KismetSystemLibrary.Delay` 0.2)
      (goto _label))))

(event `self.ReceiveTick`
  (params (DeltaSeconds :type "Float (single-precision)"))
  (if (and (`self.IsAttackRange`) (not (`self.IsAttacking`)))
    (`ActorComponent.Deactivate` (`self.CharacterMovement`))
    (`|PlayMontage` (`self.Mesh`) "/Game/Characters/Enemy_Great_Spider/Animations/AN_SpiderAttack.AN_SpiderAttack"
      (:`OnCompleted`
        (`ActorComponent.Activate` (`self.CharacterMovement`) false)))))

(fn `IsAttacking`
  (returns (ReturnValue :type Boolean))
  (return (`AnimInstance.Montage_IsPlaying` (`SkeletalMeshComponent.GetAnimInstance` (`self.Mesh`)) "/Game/Characters/Enemy_Great_Spider/Animations/AN_SpiderAttack.AN_SpiderAttack")))

(fn `IsAttackRange`
  (returns (ReturnValue :type Boolean))
  (return (< (`self.GetDistanceTo` (`GameplayStatics.GetPlayerCharacter` 0)) (`self.AttackRange`))))

(fn `UserConstructionScript`)